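; BP_PathPoints is a spline-based path actor that stores the world locations of its spline points in a PathPoints array.
; The construction script flushes persistent debug lines, rebuilds the array from the Spline component's points, and draws a short-lived debug sphere at each one.
; On BeginPlay it draws longer-lasting debug spheres at every stored point to visualize the path during play.
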(event `self.ReceiveBeginPlay`
  (for _array_element (`self.PathPoints`)
    (`KismetSystemLibrary.DrawDebugSphere` _array_element 50.0 12 (struct :`R` 0.612035 :`G` 1.0 :`A` 1.0) 60.0)))

(fn `UserConstructionScript`
  (`KismetSystemLibrary.FlushPersistentDebugLines`)
  (`KismetArrayLibrary.Array_Clear` (`self.PathPoints`))
  (for _index (range (`SplineComponent.GetNumberOfSplinePoints` (`self.Spline`)))
    (bind _returnvalue (`SplineComponent.GetLocationAtSplinePoint` (`self.Spline`) _index "World"))
    (`KismetArrayLibrary.Array_Add` (`self.PathPoints`) _returnvalue)
    (`KismetSystemLibrary.DrawDebugSphere` _returnvalue 50.0 12 (struct :`R` 0.460188 :`G` 1.0 :`A` 1.0) 10.0)))