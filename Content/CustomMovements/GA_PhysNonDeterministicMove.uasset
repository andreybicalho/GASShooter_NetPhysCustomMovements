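; Gameplay ability that runs a custom PhysNonDeterministicMove ability task, apparently a test of non-deterministic timing in custom movement.
; On activation it starts the task with an initial wait and max speed, keeping a reference to it.
; Each time the wait is reached, it prints and sets a randomly scaled wait time; a deterministic variant sits unconnected.
; Success commits the ability cost, Finish ends the ability, and Failed cancels it.
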(event `self.K2_ActivateAbility`
  (bind _returnvalue (* (`KismetMathLibrary.RandomFloat`) (`self.TimeToWait`)))
  (bind _asynctaskproxy (`GAT_ApplyPhysCustomMovement_NonDeterministicMove.PhysNonDeterministicMove` "PhysNonDeterministicMove" 3.0 300.0)
    (:`then`
      (set `self.NonDeterministicMoveAsyncTask` _asynctaskproxy))
    (:`OnReachedTime`
      ;[1 0 0.135] non-deterministic
      (`KismetSystemLibrary.PrintText` (`|FormatText` "TimeToWait: {time}" _returnvalue) true true (struct :`R` 1.0 :`G` 0.016832 :`A` 1.0) 5.0)
      (bind _nondeterministicmoveasynctask (`self.NonDeterministicMoveAsyncTask`)
        (:`then`
          (`GAT_ApplyPhysCustomMovement_NonDeterministicMove.SetWaitTime` _nondeterministicmoveasynctask _returnvalue))
        (:`else`)))
    (:`OnSuccess`
      (bind _returnvalue_2 (`self.K2_CommitAbilityCost` true))
      (if _returnvalue_2
        _))
    (:`OnFinish`
      (`self.K2_EndAbility`))
    (:`OnFailed`
      (`self.K2_CancelAbility`))))