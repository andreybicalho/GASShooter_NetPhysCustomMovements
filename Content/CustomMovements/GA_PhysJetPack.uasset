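; Gameplay ability that drives a jetpack through a PhysConstantForce custom movement task.
; After a cooldown check, the task applies JetpackForce plus the avatar's unit forward vector, with capped speed and acceleration.
; Task success commits the cost and waits for input release, which switches the character to Falling.
; Task finish ends the ability, while a failed check, task or cost commit cancels it.
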(event `self.K2_ActivateAbility`
  (bind _returnvalue (`self.K2_CheckAbilityCooldown`))
  (if _returnvalue
    (`GAT_ApplyPhysCustomMovement_ConstantForce.PhysConstantForce` "PhysConstantForce" (+ (`Actor.GetActorForwardVector` (`self.GetAvatarActorFromActorInfo`)) (`self.JetpackForce`)) 1000.0 2048.0
      (:`OnSuccess`
        (bind _returnvalue_2 (`self.K2_CommitAbilityCost` true))
        (if _returnvalue_2
          (`AbilityTask_WaitInputRelease.WaitInputRelease` true ; When the player releases Button, end the ability
            (:`OnRelease`
              (bind _ascharacter (cast `Character` (`self.GetAvatarActorFromActorInfo`)))
              (bind _charactermovement (`Character.CharacterMovement` _ascharacter))
              (`/Engine/EditorBlueprintResources/StandardMacros.IsValid` _charactermovement
                (:`Is Valid`
                  (`CharacterMovementComponent.SetMovementMode` _charactermovement "MOVE_Falling" 0)))))
          (else
            (`self.K2_CancelAbility` :!label _label))))
      (:`OnFinish`
        (`self.K2_EndAbility`))
      (:`OnFailed`
        (goto _label)))
    (else
      (goto _label))))

(event `self.K2_OnEndAbility`
  (params (bWasCancelled :type Boolean)))