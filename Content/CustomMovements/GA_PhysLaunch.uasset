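; GA_PhysLaunch is a gameplay ability that launches its avatar forward and upward through a custom PhysLaunch movement task.
; Activation checks cooldown first and cancels if it fails, otherwise launching along the avatar's forward vector with a vertical override and speed and acceleration limits.
; Cost is committed only when the launch succeeds, cancelling if that fails.
; On finish, the ability waits for client and server net sync before ending.
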(event `self.K2_ActivateAbility`
  (bind (_returnvalue_x _returnvalue_y) (`KismetMathLibrary.BreakVector` (`Actor.GetActorForwardVector` (`self.GetAvatarActorFromActorInfo`))))
  (bind _returnvalue (`self.K2_CheckAbilityCooldown`))
  (if _returnvalue
    (`GAT_ApplyPhysCustomMovement_Launch.PhysLaunch` "PhysLaunch" (`KismetMathLibrary.MakeVector` (* _returnvalue_x 300.0) (* _returnvalue_y 300.0) 600.0) false true 750.0 2048.0
      (:`OnSuccess`
        (bind _returnvalue_2 (`self.K2_CommitAbilityCost` true))
        (if (not _returnvalue_2)
          (`self.K2_CancelAbility`)))
      (:`OnFinish`
        (`AbilityTask_NetworkSyncPoint.WaitNetSync` "BothWait"
          (:`OnSync`
            (`self.K2_EndAbility`))))
      (:`OnFailed`
        (`self.K2_CancelAbility` :!label _label)))
    (else
      (goto _label))))

(event `self.K2_OnEndAbility`
  (params (bWasCancelled :type Boolean)))