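; Gameplay ability that moves the avatar along a level path using a custom PhysMoveToPoints task.
; It checks cooldown, then feeds the first BP_PathPoints actor's points to the task.
; Task success commits cost and listens for the FollowPathPoints.End event, which switches movement to Falling.
; Finish ends the ability after a server-wait net sync; failed checks or task failure cancel it.
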(event `self.K2_ActivateAbility`
  (bind _returnvalue (`self.K2_CheckAbilityCooldown`))
  (if _returnvalue
    (bind _outactors (`GameplayStatics.GetAllActorsOfClass` "/Game/CustomMovements/BP_PathPoints.BP_PathPoints_C"))
    (if (> (`KismetArrayLibrary.Array_Length` _outactors) 0)
      (`GAT_ApplyPhysCustomMovement_MoveToPoints.PhysMoveToPoints` "PhysMoveToPoints" (`/Game/CustomMovements/BP_PathPoints.PathPoints` (`|GetArrayItem` _outactors)) 100.0 3000.0
        (:`OnSuccess`
          (bind _returnvalue_2 (`self.K2_CommitAbilityCost` true))
          (if _returnvalue_2
            (`AbilityTask_WaitGameplayEvent.WaitGameplayEvent` (struct :`TagName` "GameplayEvent.FollowPathPoints.End") null true
              (:`EventReceived`
                (bind _ascharacter (cast `Character` (`self.GetAvatarActorFromActorInfo`)))
                (bind _charactermovement (`Character.CharacterMovement` _ascharacter))
                (`/Engine/EditorBlueprintResources/StandardMacros.IsValid` _charactermovement
                  (:`Is Valid`
                    (`CharacterMovementComponent.SetMovementMode` _charactermovement "MOVE_Falling" 0)))))
            (else
              (`self.K2_CancelAbility` :!label _label))))
        (:`OnFinish`
          (`AbilityTask_NetworkSyncPoint.WaitNetSync` "OnlyServerWait"
            (:`OnSync`
              (`self.K2_EndAbility`))))
        (:`OnFailed`
          (goto _label)))
      (else
        (goto _label)))
    (else
      (goto _label))))