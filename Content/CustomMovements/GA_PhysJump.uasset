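; GA_PhysJump is a gameplay ability that makes the avatar jump forward through a custom movement.
; On activation it commits the ability, then runs a PhysJump task that launches the avatar along its forward vector with an upward boost, overriding vertical velocity.
; When the task finishes it waits for client and server to sync before ending; a failed commit cancels the ability.
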(event `self.K2_ActivateAbility`
  (bind (_returnvalue_x _returnvalue_y) (`KismetMathLibrary.BreakVector` (`Actor.GetActorForwardVector` (`self.GetAvatarActorFromActorInfo`))))
  (bind _returnvalue (`self.K2_CommitAbility`))
  (if _returnvalue
    (`GSAT_ApplyPhysCustomJump.PhysJump` "PhysJump" (`KismetMathLibrary.MakeVector` (* _returnvalue_x 300.0) (* _returnvalue_y 300.0) 600.0) false true
      (:`OnFinish`
        (`AbilityTask_NetworkSyncPoint.WaitNetSync` "BothWait"
          (:`OnSync`
            (`self.K2_EndAbility`)))))
    (else
      (`self.K2_CancelAbility`))))

(event `self.K2_OnEndAbility`
  (params (bWasCancelled :type Boolean)))